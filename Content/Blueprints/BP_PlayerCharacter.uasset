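; Player character for a timed survival game, linking the character to its in-game HUD and kicking off the spawners.
; BeginPlay creates the HUD, hides the cursor, passes it the pre-start countdown, then starts every Spawner after that delay.
; Five capacity-use events forward their component's cooldown to the HUD.
; Death pauses the game and shows the cursor and death screen with the time survived.
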(event EventBeginPlay
  (bind _returnvalue (UserInterface|CreateWidget "/Game/Blueprints/HUD/WBP_InGameHUD.WBP_InGameHUD_C"))
  (bind _output_get (Variables|Default|SetMainHUD _returnvalue))
  (UserInterface|Viewport|AddtoViewport _output_get 0)
  (Variables|/Script/Engine.PlayerController|SetbShowMouseCursor (Class|GameplayStatics|GetPlayerControllerfromID) false)
  (Variables|/Game/Blueprints/HUD/WBP_InGameHUD.WBP_InGameHUD_C|SetStartTimer (Variables|Default|GetMainHUD) (Variables|Default|GetTimerBeforeStart))
  (bind _outactors (Actor|GetAllActorsOfClass "/Script/MarmotteUnrealGD.Spawner"))
  (Utilities|FlowControl|Delay (Variables|Default|GetTimerBeforeStart))
  (for _array_element _outactors
    (Class|Spawner|StartSpawner _array_element)))

(event Collision|EventActorBeginOverlap
  (params (OtherActor :type Actor%20Object%20Reference)))

(event EventTick
  (params (DeltaSeconds :type Float%20%28single-precision%29)))

(event EventOnDeath
  (bind _mainhud (Variables|Default|GetMainHUD))
  (Widget|SetVisibility (Variables|/Game/Blueprints/HUD/WBP_InGameHUD.WBP_InGameHUD_C|GetDeathScreen (Variables|Default|GetMainHUD)) "Visible")
  (Variables|/Script/Engine.PlayerController|SetbShowMouseCursor (Class|GameplayStatics|GetPlayerControllerfromID) true)
  (Game|SetGamePaused true)
  (Rendering|Components|TextRender|SetText (Variables|/Game/Blueprints/HUD/WBP_InGameHUD.WBP_InGameHUD_C|GetTimeSurviveValue _mainhud) (Utilities|Text|ToText(String) (Class|KismetStringLibrary|TimeSecondstoString (Variables|/Game/Blueprints/HUD/WBP_InGameHUD.WBP_InGameHUD_C|GetTimer _mainhud)))))

(event EventOnFirstCapacityUse
  (Default|SetFirstCapacityCD (Variables|Default|GetMainHUD) (Variables|/Script/MarmotteUnrealGD.CapacityComponent|GetCapacityCooldown (Variables|Default|GetFirstCapacityComponent))))

(event EventOnSecondCapacityUse
  (Default|SetSecondCapacityCD (Variables|Default|GetMainHUD) (Variables|/Script/MarmotteUnrealGD.CapacityComponent|GetCapacityCooldown (Variables|Default|GetSecondCapacityComponent))))

(event EventOnThirdCapacityUse
  (Default|SetThirdCapacityCD (Variables|Default|GetMainHUD) (Variables|/Script/MarmotteUnrealGD.CapacityComponent|GetCapacityCooldown (Variables|Default|GetThirdCapacityComponent))))

(event EventOnFourthCapacityUse
  (Default|SetFourthCapacityCD (Variables|Default|GetMainHUD) (Variables|/Script/MarmotteUnrealGD.CapacityComponent|GetCapacityCooldown (Variables|Default|GetFourthCapacityComponent))))

(event EventOnFifthCapacityUse
  (Default|SetFifthCapacityCD (Variables|Default|GetMainHUD) (Variables|/Script/MarmotteUnrealGD.CapacityComponent|GetCapacityCooldown (Variables|Default|GetFifthCapacityComponent))))

(fn ConstructionScript)